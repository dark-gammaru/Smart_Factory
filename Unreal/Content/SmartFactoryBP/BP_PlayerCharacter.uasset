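; Player character for SmartFactory that reacts to the game's night and morning transitions.
; On BeginPlay it binds custom events to the night and morning delegates on SmartFactoryGameInstance.
; Night disables the character's input, and morning teleports it to the location and rotation of PlayerStartRef, then re-enables input.
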(event Custom|Night%20Event
  (Input|DisableInput 0))

(event Custom|Morning%20Event
  (bind _playerstartref (Variables|Default|GetPlayerStartRef))
  (Transformation|SetActorLocationAndRotation (Transformation|GetActorLocation _playerstartref) (Transformation|GetActorRotation _playerstartref) false true)
  (Input|EnableInput 0))

(event EventBeginPlay
  (bind _assmart_factory_game_instance (Utilities|Casting|CastToSmartFactoryGameInstance (Game|GetGameInstance)))
  (EventDispatchers|BindEventtoNightDelegate _assmart_factory_game_instance (delegate Custom|Night%20Event))
  (EventDispatchers|BindEventtoMorningDelegate _assmart_factory_game_instance (delegate Custom|Morning%20Event)))

(fn ConstructionScript)