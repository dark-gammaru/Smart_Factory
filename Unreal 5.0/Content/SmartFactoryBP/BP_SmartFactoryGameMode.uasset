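; Game mode for the SmartFactory game that sets up its screen UI and handles game over.
; On BeginPlay it shows the factory widget and an eyelid widget whose close animation plays in reverse as an eye-opening intro.
; It then binds GameOverEvent to the SmartFactory game instance's game-over delegate, which adds the death screen widget to the viewport.
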(event Custom|Game%20Over%20Event
  (bind _returnvalue (UserInterface|CreateWidget "/Game/SmartFactoryBP/BP_DeathScreen.BP_DeathScreen_C"))
  (UserInterface|Viewport|AddtoViewport _returnvalue 0))

(event EventBeginPlay
  (bind _returnvalue (UserInterface|CreateWidget "/Game/SmartFactoryBP/BP_SmartFactoryWidget.BP_SmartFactoryWidget_C"))
  (UserInterface|Viewport|AddtoViewport _returnvalue 0)
  (bind _returnvalue_2 (UserInterface|CreateWidget "/Game/SmartFactoryBP/BP_Eyelids.BP_Eyelids_C"))
  (UserInterface|Animation|PlayAnimation _returnvalue_2 (Variables|/Game/SmartFactoryBP/BP_Eyelids.BP_Eyelids_C|GetCloseEye _returnvalue_2) 0.0 1 "Reverse" 1.0 false)
  (UserInterface|Viewport|AddtoViewport _returnvalue_2 0)
  (bind _assmart_factory_game_instance (Utilities|Casting|CastToSmartFactoryGameInstance (Game|GetGameInstance)))
  (EventDispatchers|BindEventtoGameOverDelegate _assmart_factory_game_instance (delegate Custom|Game%20Over%20Event)))

(fn ConstructionScript)