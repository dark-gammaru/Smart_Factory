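; BP_PlayerCharacter is the smart factory player character, whose input follows the game's night and morning cycle.
; On BeginPlay it binds to the night and morning delegates on SmartFactoryGameInstance, disabling input at night and re-enabling it in the morning.
; A WidgetInteraction component receives left mouse press, release and wheel scroll, so the player can operate 3D widgets in the world.
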(event Custom|Night%20Event
  (Input|DisableInput 0))

(event Custom|Morning%20Event
  (Input|EnableInput 0))

(event EventBeginPlay
  (bind _assmart_factory_game_instance (Utilities|Casting|CastToSmartFactoryGameInstance (Game|GetGameInstance)))
  (EventDispatchers|BindEventtoNightDelegate _assmart_factory_game_instance (delegate Custom|Night%20Event))
  (EventDispatchers|BindEventtoMorningDelegate _assmart_factory_game_instance (delegate Custom|Morning%20Event)))

(event Input|MouseEvents|MouseWheelAxis
  (params (AxisValue :type Float%20%28single-precision%29))
  ;[1 1 1] 3D Widget 상호작용 포인터 이벤트 등록
  (Class|WidgetInteractionComponent|ScrollWheel (Variables|Default|GetWidgetInteraction) AxisValue))

(event Input|MouseEvents|LeftMouseButton
  (params (Key :type Key%20Structure :default "None"))
  (bind _widgetinteraction (Variables|Default|GetWidgetInteraction))
  ;[1 1 1] 3D Widget 상호작용 포인터 이벤트 등록
  (:Pressed
    (Class|WidgetInteractionComponent|PressPointerKey _widgetinteraction "LeftMouseButton"))
  (:Released
    (Class|WidgetInteractionComponent|ReleasePointerKey _widgetinteraction "LeftMouseButton")))

(fn ConstructionScript)