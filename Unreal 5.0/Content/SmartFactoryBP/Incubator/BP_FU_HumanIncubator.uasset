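; Human incubator actor that serves as the ending set piece of the smart factory game, closing the player in and then quitting.
; On the GameClear delegate it moves and triggers the WallManager's destructible chaos volume at its location, then rises and swings its door open.
; Capsule overlap runs a one-shot scripted sequence of chained timelines and delays: door, shutter, lights off, ending voice and sounds, then QuitGame.
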(event OnComponentBeginOverlap(Capsule)
  (params (OverlappedComponent :type Primitive%20Component%20Object%20Reference) (OtherActor :type Actor%20Object%20Reference) (OtherComp :type Primitive%20Component%20Object%20Reference) (OtherBodyIndex :type Integer) (bFromSweep :type Boolean) (SweepResult :type Hit%20Result%20Structure%20%28by%20ref%29))
  (bind _asplayer_character (Utilities|Casting|CastToPlayerCharacter OtherActor))
  (Variables|/Script/Unreal.PlayerCharacter|SetMovable _asplayer_character false)
  (EventDispatchers|UnbindallEventsfromOnComponentBeginOverlap OverlappedComponent)
  (Utilities|FlowControl|Delay 2.0)
  (Audio|PlaySoundatLocation "/Game/Resources/Sound/Incubator/SE_IncubatorDoor.SE_IncubatorDoor" (Transformation|GetActorLocation) "0, 0, 0" 1.0 1.0 0.0 "/Game/Resources/Sound/BasicAttenuation.BasicAttenuation" 0 0 0)
  (bind _alpha (Timeline|Timeline_0 PlayFromStart)
    (:Update
      (Transformation|SetRelativeRotation (Variables|Default|GetSM_FU_humanIncubatorDoor) (Math|Rotator|Lerp(Rotator) "0,180.000000, 0" "0, 0, 0" _alpha) false false))
    (:Finished
      (Variables|/Script/Unreal.PlayerCharacter|SetMovable _asplayer_character true)
      (Audio|PlaySoundatLocation "/Game/Resources/Sound/Incubator/SE_IncubatorDoor.SE_IncubatorDoor" (Transformation|GetActorLocation) "0, 0, 0" 1.0 1.0 0.0 "/Game/Resources/Sound/BasicAttenuation.BasicAttenuation" 0 0 0)
      (bind _alpha_2 (Timeline|Timeline_1 PlayFromStart)
        (:Update
          (Transformation|SetRelativeScale3D (Variables|Default|GetShutter) (Math|Vector|Lerp(Vector) "1.000000,1.000000,0.000000" "1.000000,1.000000,1.000000" _alpha_2)))
        (:Finished
          (Utilities|FlowControl|Delay 2.0)
          (Components|DestroyComponent (Variables|Default|GetSpotLight1))
          (Components|DestroyComponent (Variables|Default|GetSpotLight2))
          (Rendering|Material|SetMaterial (Variables|Debug|GetStaticMeshComponent) 3 "/Game/Resources/GenralMaterials/MI_Plastic_Black.MI_Plastic_Black")
          (Audio|PlaySound2D "/Game/Resources/Sound/Incubator/SE_LightOff.SE_LightOff" 1.0 1.0 0.0 0 0 false)
          (Utilities|FlowControl|Delay 3.0)
          (Audio|PlaySound2D "/Game/Resources/Sound/TTS/SE_TTS_Ending.SE_TTS_Ending" 1.0 1.0 0.0 0 0 false)
          (Utilities|FlowControl|Delay 1e+01)
          (Audio|PlaySound2D "/Game/Resources/Sound/Incubator/SE_IncubatorManufactureAnimal.SE_IncubatorManufactureAnimal" 1.0 1.0 0.0 0 0 false)
          (Utilities|FlowControl|Delay 2.0)
          (Game|QuitGame 0 "Quit" false))))))

(event Custom|Game%20Clear
  (bind _asbp_smart_factory_game_instance (Utilities|Casting|CastToBP_SmartFactoryGameInstance (Game|GetGameInstance)))
  (Transformation|SetActorScale3D (Variables|/Script/Unreal.WallManager|GetChaosVolume (Actor|GetComponentbyClass (Variables|/Script/Unreal.SmartFactoryGameInstance|GetManager _asbp_smart_factory_game_instance) "/Script/Unreal.WallManager")) "5.000000,5.000000,100.000000")
  (Transformation|SetActorLocation (Variables|/Script/Unreal.WallManager|GetChaosVolume (Actor|GetComponentbyClass (Variables|/Script/Unreal.SmartFactoryGameInstance|GetManager _asbp_smart_factory_game_instance) "/Script/Unreal.WallManager")) (Transformation|GetActorLocation) true false)
  (Class|ChaosDestructionTriggerVolume|MakeDestructable (Variables|/Script/Unreal.WallManager|GetChaosVolume (Actor|GetComponentbyClass (Variables|/Script/Unreal.SmartFactoryGameInstance|GetManager _asbp_smart_factory_game_instance) "/Script/Unreal.WallManager")))
  (Variables|Default|SetFirstLocationSaved (Transformation|GetActorLocation))
  (bind _alpha (Timeline|Incubator%20Raise PlayFromStart)
    (:Update
      (Transformation|SetActorLocation (Math|Vector|Lerp(Vector) (Variables|Default|GetFirstLocationSaved) (+ (Variables|Default|GetFirstLocationSaved) "0,0,241.000000") _alpha) false false))
    (:Finished
      (Audio|PlaySoundatLocation "/Game/Resources/Sound/Incubator/SE_IncubatorDoor.SE_IncubatorDoor" (Transformation|GetActorLocation) "0, 0, 0" 1.0 1.0 0.0 "/Game/Resources/Sound/BasicAttenuation.BasicAttenuation" 0 0 0)
      (bind _alpha_2 (Timeline|Door%20Rotate PlayFromStart)
        (:Update
          (Transformation|SetRelativeRotation (Variables|Default|GetSM_FU_humanIncubatorDoor) (Math|Rotator|Lerp(Rotator) "0, 0, 0" "0.000000,179.000000,0.000000" _alpha_2 true) false false))))))

(event EventBeginPlay
  (bind _asbp_smart_factory_game_instance (Utilities|Casting|CastToBP_SmartFactoryGameInstance (Game|GetGameInstance)))
  (EventDispatchers|BindEventtoGameClearDelegate _asbp_smart_factory_game_instance (delegate Custom|Game%20Clear)))

(fn ConstructionScript)