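; Plant incubator Blueprint for the smart factory that animates its door, shutters and spotlight around commodity processing.
; PutCommodity closes the door, lights the spotlight and initializes the UI with the first attached actor.
; Manufacture and AbortCommodity close the shutters, call the matching Incubator function, then after a delay reopen shutters and door while switching off the light.
; Timelines drive the motion, lerping scale on four shutter meshes and rotation on the door.
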(event EventManufacture
  (CallFunction|PlayDoorSound)
  (bind _alpha (Timeline|CloseShutterTimeline PlayFromStart)
    (:Update
      (CallFunction|MoveShutter _alpha false))
    (:Finished
      (Class|Incubator|Manufacture (Variables|Default|GetIncubator))
      (Audio|PlaySoundatLocation "/Game/Resources/Sound/Incubator/SE_IncubatorManufacturePlant.SE_IncubatorManufacturePlant" (Transformation|GetActorLocation) "0, 0, 0" 1.0 1.0 0.0 "/Game/Resources/Sound/BasicAttenuation.BasicAttenuation" 0 0 0)
      (Utilities|FlowControl|Delay 2.0)
      (CallFunction|PlayDoorSound)
      (bind _alpha_2 (Timeline|OpenShutterTimeline PlayFromStart)
        (:Update
          (CallFunction|MoveShutter _alpha_2 true))
        (:Finished
          (CallFunction|PlayDoorSound)
          (bind _alpha_3 (Timeline|OpenDoorTimeline PlayFromStart)
            (:Update
              (CallFunction|MoveDoor _alpha_3 true)
              (CallFunction|ControlLight (Variables|Default|GetSpotLight) _alpha_3 false))))))))

(event EventAbortCommodity
  (CallFunction|PlayDoorSound)
  (bind _alpha (Timeline|Timeline_1 PlayFromStart)
    (:Update
      (CallFunction|MoveShutter _alpha false))
    (:Finished
      (Class|Incubator|AbortCommodity (Variables|Default|GetIncubator))
      (Utilities|FlowControl|Delay 1.0)
      (CallFunction|PlayDoorSound)
      (bind _alpha_2 (Timeline|Timeline_2 PlayFromStart)
        (:Update
          (CallFunction|MoveShutter _alpha_2 true))
        (:Finished
          (CallFunction|PlayDoorSound)
          (bind _alpha_3 (Timeline|Timeline_0 PlayFromStart)
            (:Update
              (CallFunction|MoveDoor _alpha_3 true)
              (CallFunction|ControlLight (Variables|Default|GetSpotLight) _alpha_3 false))))))))

(event EventPutCommodity
  (CallFunction|PlayDoorSound)
  (bind _alpha (Timeline|CloseDoorTimeline PlayFromStart)
    (:Update
      (CallFunction|MoveDoor _alpha false)
      (CallFunction|ControlLight (Variables|Default|GetSpotLight) _alpha true))
    (:Finished
      (CallFunction|InitializeUI (Utilities|Array|Get(acopy) (Actor|GetAttachedActors true false))))))

(fn ConstructionScript
  (Variables|Default|SetShutterArray (Utilities|Array|MakeArray (Variables|Default|GetSM_FU_typePshutter1) (Variables|Default|GetSM_FU_typePshutter2) (Variables|Default|GetSM_FU_typePshutter3) (Variables|Default|GetSM_FU_typePshutter4))))

(fn MoveShutter
  (params (Alpha :type Float%20%28double-precision%29) (IsOpen :type Boolean))
  (for _array_element (Variables|Default|GetShutterArray)
    (Transformation|SetRelativeScale3D _array_element (Math|Vector|Lerp(Vector) (Variables|Default|GetShutterClosedVector) (Variables|Default|GetShutterOpenedVector) (select IsOpen Alpha (- 1.0 Alpha))))))

(fn MoveDoor
  (params (Alpha :type Float%20%28double-precision%29) (IsOpen :type Boolean))
  (Transformation|SetRelativeRotation (Variables|Default|GetSM_FU_typePdoor) (Math|Rotator|Lerp(Rotator) (Variables|Default|GetClosedRotator) (Variables|Default|GetOpenedRotator) (select IsOpen Alpha (- 1.0 Alpha))) false false))