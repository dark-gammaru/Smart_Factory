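; BP_HologramAnimalIncubator is the hologram preview used to check whether an animal incubator can be placed.
; The construction script applies a dynamic hologram material to the mesh, and begin and end overlap events maintain a list of blocking actors.
; Each tick sets the material's availability parameter from that list alone.
; It also writes IsConstructable on the player's PlayerInteraction component, additionally requiring the hologram to be above a minimum height.
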(event EventTick
  (params (DeltaSeconds :type Float%20%28single-precision%29))
  (bind _overlappingactors (Variables|Default|GetOverlappingActors))
  (bind _material (Variables|Default|GetMaterial))
  (bind _returnvalue (Utilities|Array|Length _overlappingactors))
  (bind _returnvalue_2 (== _returnvalue 0))
  (if _returnvalue_2
    (Rendering|Material|SetScalarParameterValue _material "IsAvailiable" 1.0 :!class /Script/Engine.MaterialInstanceDynamic)
    (else
      (Rendering|Material|SetScalarParameterValue _material "IsAvailiable" 0.0 :!class /Script/Engine.MaterialInstanceDynamic)))
  (Variables|/Script/Unreal.PlayerInteraction|SetbIsConstructable (Actor|GetComponentbyClass (Game|GetPlayerCharacter 0) "/Script/Unreal.PlayerInteraction") (and (< -1e+02 (.Z (Math|Vector|BreakVector (Transformation|GetActorLocation)))) _returnvalue_2)))

(event Collision|EventActorBeginOverlap
  (params (OtherActor :type Actor%20Object%20Reference))
  (Utilities|Array|Add (Variables|Default|GetOverlappingActors) OtherActor))

(event Collision|EventActorEndOverlap
  (params (OtherActor :type Actor%20Object%20Reference))
  (Utilities|Array|RemoveItem (Variables|Default|GetOverlappingActors) OtherActor))

(fn ConstructionScript
  (bind _returnvalue (Rendering|Material|CreateDynamicMaterialInstance (Variables|Debug|GetStaticMeshComponent) 0 "/Game/Resources/GenralMaterials/MA_GE_Hologram.MA_GE_Hologram" "None" :!class /Script/Engine.PrimitiveComponent))
  (Variables|Default|SetMaterial _returnvalue)
  (Rendering|Material|SetMaterial (Variables|Debug|GetStaticMeshComponent) 0 _returnvalue))