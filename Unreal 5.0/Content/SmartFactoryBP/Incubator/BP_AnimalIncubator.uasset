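; Animal incubator for a smart factory that animates a commodity, its first attached actor, through loading and manufacturing.
; PutCommodity closes the doors, lights the interior, initializes the UI, attaches six cables to the commodity and moves it to the center.
; Manufacture closes the shutter, calls the Incubator, resets the cables, then reopens shutter and doors.
; Chained timelines drive all motion, with pass-through GetTmpVector capturing lerp endpoints beforehand.
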(event Custom|PutCommodity
  (bind _outactors (Actor|GetAttachedActors true false))
  (bind _output (Utilities|Array|Get(acopy) _outactors))
  (bind _alpha (Timeline|CloseDoorTimeline PlayFromStart)
    (:Update
      (CallFunction|MoveDoor _alpha false)
      (CallFunction|ControlLight (Variables|Default|GetRectLightInside) _alpha true))
    (:Finished
      (CallFunction|InitializeUI _output)
      ;[1 1 1] Move Cable Spheres To Commodity
      (bind _savedvector (CallFunction|GetTmpVector (Transformation|GetActorLocation _output)))
      (bind _alpha_2 (Timeline|CableAttachTimeline PlayFromStart)
        (:Update
          (for (_array_element _array_index) (Variables|Default|GetCableSpheres)
            (Transformation|SetWorldLocation _array_element (Math|Vector|Lerp(Vector) (Utilities|Array|Get(acopy) (Variables|Default|GetCableSphereInitialLocations) _array_index) _savedvector _alpha_2) false false)))
        (:Finished
          ;[1 1 1] Attach Cables To Commodity
          (for _array_element_2 (Variables|Default|GetCables)
            (Class|CableComponent|SetAttachEndto _array_element_2 _output "None" "None"))
          ;[1 1 1] Move Commodities To Center
          (bind _savedvector_2 (CallFunction|GetTmpVector (Transformation|GetActorLocation _output)))
          (bind _savedvector_3 (CallFunction|GetTmpVector (+ (Variables|Default|GetAnimalPosition) (Transformation|GetActorLocation))))
          (bind _alpha_3 (Timeline|MoveCommodityTimeline PlayFromStart)
            (:Update
              (Transformation|SetActorLocation _output (Math|Vector|Lerp(Vector) _savedvector_2 _savedvector_3 _alpha_3) false false)
              (for _array_element_3 (Variables|Default|GetCableSpheres)
                (Transformation|SetWorldLocation _array_element_3 (Math|Vector|Lerp(Vector) _savedvector_2 _savedvector_3 _alpha_3) false false)))))))))

(event Custom|Manufacture
  (bind _alpha (Timeline|CloseShutterTimeline PlayFromStart)
    (:Update
      (CallFunction|MoveShutter _alpha false))
    (:Finished
      (Class|Incubator|Manufacture (Variables|Default|GetIncubator))
      (CallFunction|ResetCable)
      (Utilities|FlowControl|Delay 3.0)
      (bind _alpha_2 (Timeline|OpenShutterTimeline PlayFromStart)
        (:Update
          (CallFunction|MoveShutter _alpha_2 true))
        (:Finished
          (bind _alpha_3 (Timeline|OpenDoorTimeline PlayFromStart)
            (:Update
              (CallFunction|MoveDoor _alpha_3 true)
              (CallFunction|ControlLight (Variables|Default|GetRectLightInside) _alpha_3 false))))))))

(fn ConstructionScript
  (Variables|Default|SetCables (Utilities|Array|MakeArray (Variables|Default|GetCable) (Variables|Default|GetCable1) (Variables|Default|GetCable2) (Variables|Default|GetCable3) (Variables|Default|GetCable4) (Variables|Default|GetCable5)))
  (Variables|Default|SetCableSpheres (Utilities|Array|MakeArray (Variables|Default|GetCableSphere) (Variables|Default|GetCable1Sphere) (Variables|Default|GetCable2Sphere) (Variables|Default|GetCable3Sphere) (Variables|Default|GetCable4Sphere) (Variables|Default|GetCable5Sphere)))
  (for (_array_element _array_index) (Variables|Default|GetCableSpheres)
    (Utilities|Array|SetArrayElem (Variables|Default|GetCableSphereInitialLocations) _array_index (Transformation|GetWorldLocation _array_element))))

(fn MoveDoor
  (params (Alpha :type Float%20%28double-precision%29) (IsOpen :type Boolean))
  (bind _returnvalue (- 1.0 Alpha))
  (bind _returnvalue_2 (select IsOpen Alpha _returnvalue))
  (Transformation|SetRelativeLocation (Variables|Default|GetSM_FU_typeAdoor1) (Math|Vector|Lerp(Vector) (Variables|Default|GetDoor1ClosedLoc) (Variables|Default|GetDoor1OpenedLoc) _returnvalue_2) false false)
  (Transformation|SetRelativeLocation (Variables|Default|GetSM_FU_typeAdoor2) (Math|Vector|Lerp(Vector) (Variables|Default|GetDoor2ClosedLoc) (Variables|Default|GetDoor2OpenedLoc) _returnvalue_2) false false))

(fn MoveShutter
  (params (Alpha :type Float%20%28double-precision%29) (IsOpen :type Boolean))
  (Transformation|SetRelativeScale3D (Variables|Default|GetShutter) (Math|Vector|Lerp(Vector) (Variables|Default|GetShutterClosedVector) (Variables|Default|GetShutterOpenedVector) (select IsOpen Alpha (- 1.0 Alpha)))))

(fn ResetCable
  (for (_array_element _array_index) (Variables|Default|GetCables)
    (Class|CableComponent|SetAttachEndto _array_element 0 (Utilities|String|StringToName (Utilities|GetObjectName (Utilities|Array|Get(acopy) (Variables|Default|GetCableSpheres) _array_index))) "None"))
  (for (_array_element_2 _array_index_2) (Variables|Default|GetCableSphereInitialLocations)
    (Transformation|SetWorldLocation (Utilities|Array|Get(acopy) (Variables|Default|GetCableSpheres) _array_index_2) _array_element_2 false false)))

(fn GetTmpVector
  (params (Vector :type Vector))
  (return Vector))