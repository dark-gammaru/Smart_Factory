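; BP_IncubatorBase is the base incubator actor in the smart factory, providing a UI widget, lighting, sound and destruction helpers.
; BeginPlay initializes the BP_PA_Incubator widget, and InitializeUI fills it from the CommodityTable row matching the passed actor's Commodity component name.
; ControlLight blends intensity and color temperature by alpha, while other helpers play door sounds or make the Incubator destructible.
; Manufacture, AbortCommodity and PutCommodity are empty events here.
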(event Custom|Manufacture)

(event Custom|AbortCommodity)

(event Custom|PutCommodity)

(event EventBeginPlay
  (bind _asbp_pa_incubator (Utilities|Casting|CastToBP_PA_Incubator (UserInterface|GetUserWidgetObject (Variables|Default|GetWidget))))
  (Default|Initialize _asbp_pa_incubator (Variables|Default|GetIncubator)))

(fn ConstructionScript)

(fn ControlLight
  (params (Light :type Light%20Component%20Object%20Reference) (Alpha :type Float%20%28double-precision%29) (IsTurnOn :type Boolean))
  (bind _returnvalue (- 1.0 Alpha))
  (bind _returnvalue_2 (select IsTurnOn Alpha _returnvalue))
  (Rendering|Components|Light|SetIntensity Light (Math|Float|Lerp 2e+02 2e+03 _returnvalue_2))
  (Class|LightComponent|SetTemperature Light (Math|Float|Lerp 6.5e+03 2e+03 _returnvalue_2)))

(fn InitializeUI
  (params (NewParam :type Actor%20Object%20Reference))
  (bind _returnvalue (Class|HoldableObject|GetName (Actor|GetComponentbyClass NewParam "/Script/Unreal.Commodity")))
  (bind _asbp_pa_incubator (Utilities|Casting|CastToBP_PA_Incubator (UserInterface|GetUserWidgetObject (Variables|Default|GetWidget))))
  (bind _returnvalue_2 (Utilities|GetDataTableRow "/Game/SmartFactoryBP/HoldableObjects/CommodityTable.CommodityTable" (Utilities|String|StringToName _returnvalue))
    (:then
      (Default|SetCommodity _asbp_pa_incubator (.image _returnvalue_2) _returnvalue (.scientificname _returnvalue_2) (.information _returnvalue_2) (.growthtime _returnvalue_2)))))

(fn DestroyIncubator
  (Class|ChaosDestructable|MakeDestructable (Variables|Default|GetIncubator))
  (Audio|PlaySoundatLocation "/Game/Resources/Sound/Incubator/SE_IncubatorDestroyed.SE_IncubatorDestroyed" (Transformation|GetActorLocation) "0, 0, 0" 1.0 1.0 0.0 "/Game/Resources/Sound/BasicAttenuation.BasicAttenuation" 0 0 0))

(fn PlayDoorSound
  (Audio|PlaySoundatLocation "/Game/Resources/Sound/Incubator/SE_IncubatorDoor.SE_IncubatorDoor" (Transformation|GetActorLocation) "0, 0, 0" 1.0 1.0 0.0 "/Game/Resources/Sound/BasicAttenuation.BasicAttenuation" 0 0 0))